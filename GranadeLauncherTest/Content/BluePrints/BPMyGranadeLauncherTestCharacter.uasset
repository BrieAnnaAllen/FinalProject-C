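; Test character Blueprint, named for a grenade launcher, whose graph handles a toggleable dialog UI.
; BeginPlay creates a BPDialogUIWidget for the first player controller and keeps it as UI.
; ToggleUI either passes the character's Questions to the widget and shows it with cursor and game-and-UI input, or removes it and restores game-only input.
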(event EventBeginPlay
  (bind _returnvalue (UserInterface|CreateWidget "/Game/BluePrints/BPDialogUIWidget.BPDialogUIWidget_C" (Game|GetPlayerController 0)))
  (Variables|Default|SetUI _returnvalue))

(event Collision|EventActorBeginOverlap
  (params (OtherActor :type Actor%20Object%20Reference)))

(event EventTick
  (params (DeltaSeconds :type Float%20%28single-precision%29)))

(event EventToggleUI
  (bind _returnvalue (Game|GetPlayerController 0))
  (bind _returnvalue_2 (Game|GetPlayerController 0))
  (bind _ui (Variables|Default|GetUI))
  (Utilities|IsValid _ui
    (:Is%20Valid
      (if (UserInterface|Viewport|IsinViewport _ui)
        (Input|SetInputModeGameOnly _returnvalue_2)
        (Variables|/Script/Engine.PlayerController|SetbShowMouseCursor _returnvalue_2 false)
        (Widget|RemovefromParent (Variables|Default|GetUI))
        (else
          (Variables|/Script/GranadeLauncherTest.DialogUI|SetQuestions _ui (Variables|Default|GetQuestions))
          (Class|DialogUI|Show _ui)
          (Variables|/Script/Engine.PlayerController|SetbShowMouseCursor _returnvalue true)
          (Input|SetInputModeGameandUI _returnvalue (Variables|Default|GetUI) "DoNotLock" true))))))

(fn ConstructionScript)